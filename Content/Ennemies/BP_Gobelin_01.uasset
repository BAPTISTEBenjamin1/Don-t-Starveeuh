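; Goblin enemy Character that roams random reachable points, chases the player on sight through PawnSensing and attacks on arrival.
; An attack montage notify briefly enables weapon collision, which deals damage and stun through an interface.
; Incoming damage updates a health bar widget and triggers a dynamic-material Fresnel flash; death spawns loot.
; Ally call-for-help via overlap trigger is marked uncertain; knockback is an unfinished, uncalled launch.
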(event `self.ReceiveBeginPlay`
  (`self.Roaming`)
  (`self.CreateParameterValue`)
  (bind _asui_jauge_ennemies (cast `/Game/UI/Jauges/UI_JaugeEnnemies` (`WidgetComponent.GetUserWidgetObject` (`self.Health_Bar`))))
  (bind _output_get (set `self.As Jauge Ennemies` _asui_jauge_ennemies))
  (set `self.Health_Max` (`self.Health`))
  (set `/Game/UI/Jauges/UI_JaugeEnnemies.HealthBar` (`self.Health`) _output_get)
  (set `/Game/UI/Jauges/UI_JaugeEnnemies.HealthBar_Max` (`self.Health_Max`) _output_get))

(event `CreateParameterValue`
  ;[1 1 1] Create Dynamic Material
  (bind _returnvalue (`KismetMaterialLibrary.CreateDynamicMaterialInstance` (`PrimitiveComponent.GetMaterial` (`self.Mesh`) 0)))
  (bind _output_get (set `self.DynamicParameter` _returnvalue))
  (`PrimitiveComponent.SetMaterial` (`self.Mesh`) 0 _output_get))

(event `Roaming`
  ;[0.4325 1 0.4263] Roaming
  (set `CharacterMovementComponent.MaxWalkSpeed` (`self.Roaming_Walk_Speed`) (`self.CharacterMovement`))
  (`|AIMoveTo` self (`NavigationSystemV1.K2_GetRandomReachablePointInRadius` (`SceneComponent.K2_GetComponentLocation` (`self.Mesh`)) (`self.Roaming_Surface`) null null) null
    (:`OnSuccess`
      (`KismetSystemLibrary.Delay` (`KismetMathLibrary.RandomFloatInRange` 0.5 1.5))
      (`self.Roaming`))))

(event `Feedback__Fresnel`
  ;[0.05469 0.1148 0.2188] FeedBackFresnel
  (bind (_direction _base) (`Timeline|Timeline` :!via `PlayFromStart`)
    (:`Update`
      _)
    (:`Finished`
      _))
  (`MaterialInstanceDynamic.SetScalarParameterValue` (`self.DynamicParameter`) (`self.ParameterName`) _base))

(event `CreateWidget`
  ;[1 1 1] Add_Widgets_Jauges
  (`AddComponent|NODE_AddWidgetComponent-0`))

(event `KnockBack`
  ;[1 1 1] ///En chantier /// Knock Back
  (`self.LaunchCharacter` (0.0 0.0 1000.0)))

(event `self.PawnSensing.OnSeePawn`
  (params (Pawn :type "Pawn Object Reference"))
  ;[1 0.5541 0.1279] Chasing
  (`self.Chasing`)
  (if (`PrimitiveComponent.IsOverlappingActor` (`self.CallHelp_Trigger`) (`self.Ref_Ally`))
    (message `/Game/Interfaces/EnnemytoEnnemy.CallHelp` (`self.Ref_Ally`) true)))

(event `Chasing`
  ;[1 0.5541 0.1279] Chasing
  (`|ExecutionSequence`
    (:`then_0`
      (set `CharacterMovementComponent.MaxWalkSpeed` (`self.Chase_Walk_Speed`) (`self.CharacterMovement`))
      (`|AIMoveTo` self (0.0 0.0 0.0) (`GameplayStatics.GetPlayerCharacter` 0)
        (:`OnSuccess`
          (`self.Attack`)
          (`KismetSystemLibrary.PrintString` "Attrapé"))))
    (:`then_1`
      (`KismetSystemLibrary.RetriggerableDelay` 0.1)
      (`self.Roaming`))))

(event `Weapon Enable`
  ;[1 1 1] Enable_Weapon
  (`PrimitiveComponent.SetCollisionEnabled` (`self.Weapon`) "QueryOnly")
  (`KismetSystemLibrary.Delay` 0.001)
  (`PrimitiveComponent.SetCollisionEnabled` (`self.Weapon`) "NoCollision"))

(event `Attack`
  ;[1 0.2425 0.1027] Attack
  (`CharacterMovementComponent.DisableMovement` (`self.CharacterMovement`))
  (`KismetSystemLibrary.Delay` (`self.ReactionAttack`))
  (`|PlayMontage` (`self.Mesh`) "/Game/Ennemies/Gobelin/Animations/attack_01.attack_01"
    (:`then`
      (`KismetSystemLibrary.Delay` (`self.Attack_CooldDown`))
      (`CharacterMovementComponent.SetMovementMode` (`self.CharacterMovement`) "MOVE_Walking" 0))
    (:`OnNotifyBegin`
      (`self.Weapon Enable`))))

(event `self.Weapon.OnComponentBeginOverlap`
  (params (OverlappedComponent :type "PrimitiveComponent Object Reference") (OtherActor :type "Actor Object Reference") (OtherComp :type "PrimitiveComponent Object Reference") (OtherBodyIndex :type Integer) (bFromSweep :type Boolean) (SweepResult :type "HitResult Structure (by ref)"))
  ;[1 0.2339 0 0.5] Deal_Damages
  (if (`KismetSystemLibrary.DoesImplementInterface` OtherActor "/Game/Interfaces/BP_Interfaces_Ennemy.BP_Interfaces_Ennemy_C")
    (message `/Game/Interfaces/BP_Interfaces_Ennemy.Deal_DamagestoPlayer` OtherActor (`self.Damages`) (`self.StunAttackAmount`))))

(event `/Game/Interfaces/BP_Interfaces_Ennemy.Deal_Damages_To_Ennemy`
  (params (Damages :type "Float (double-precision)"))
  (bind _health (`self.Health`))
  (bind _returnvalue (- _health Damages))
  ;[1 0.08723 0] Take_Damages
  (set `/Game/UI/Jauges/UI_JaugeEnnemies.HealthBar` _returnvalue (`self.As Jauge Ennemies`))
  (bind _output_get (set `self.Health` _returnvalue))
  (`KismetSystemLibrary.PrintString` (`KismetStringLibrary.Conv_DoubleToString` _output_get) true true (struct :`G` 1.0 :`B` 0.381067 :`A` 1.0) 1.0)
  (`self.Feedback__Fresnel`)
  (`GameplayStatics.PlaySoundAtLocation` "/Engine/VREditor/Sounds/UI/Dockable_Window_Pick_Up.Dockable_Window_Pick_Up" (`SceneComponent.K2_GetComponentLocation` (`self.CapsuleComponent`)) (struct) 1.0 1.0 0.0 null null null null)
  (if (<= _health 0.0)
    (`self.Ennemy_Dead`)))

(event `self.CallHelp_Trigger.OnComponentBeginOverlap`
  (params (OverlappedComponent :type "PrimitiveComponent Object Reference") (OtherActor :type "Actor Object Reference") (OtherComp :type "PrimitiveComponent Object Reference") (OtherBodyIndex :type Integer) (bFromSweep :type Boolean) (SweepResult :type "HitResult Structure (by ref)"))
  ;[1 1 1] Je sais pas vraiment si ca marche :/
  (if (`KismetSystemLibrary.DoesImplementInterface` OtherActor "/Game/Interfaces/EnnemytoEnnemy.EnnemytoEnnemy_C")
    (set `self.Ref_Ally` OtherActor)))

(event `Ennemy_Dead`
  ;[0 0 0] Ennemy Dead
  (`GameplayStatics.PlaySound2D` "/Engine/VREditor/Sounds/UI/Dockable_Window_Close.Dockable_Window_Close" 1.0 1.0 0.0 null null)
  (`self.Spawn_Loot`)
  (`self.K2_DestroyActor`))

(event `Spawn_Loot`
  (bind _returnvalue (`SceneComponent.K2_GetComponentLocation` (`self.Weapon`)))
  ;[1 0.7128 0 0.5] Loot
  (`|SpawnActorFromClass` "/Game/Collectibles/BP_Graisse_de_Connard.BP_Graisse_de_Connard_C" (`KismetMathLibrary.Conv_VectorToTransform` _returnvalue) "Undefined" "MultiplyWithRoot" null null)
  (`KismetSystemLibrary.PrintString` "Drawn SPhere ??")
  (`KismetSystemLibrary.DrawDebugSphere` _returnvalue 60.0 12 (struct :`R` 1.0 :`G` 0.123857 :`A` 1.0) 1.0 2.0)
  (`KismetSystemLibrary.PrintString` "Ca draw"))

(event `/Game/Interfaces/EnnemytoEnnemy.CallHelp`
  (params (`CallHelpp?` :type Boolean))
  (if `CallHelpp?`
    (`|AIMoveTo` self (0.0 0.0 0.0) (`GameplayStatics.GetPlayerCharacter` 0))))

(fn `UserConstructionScript`)