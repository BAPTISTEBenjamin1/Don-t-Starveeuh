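; Campfire actor that acts as a camp safe zone, healing actors in its area while lit and damaging the player outside its dome at night.
; A delayed loop drains fire health, scaling light, material emissive and a UI bar until the fire goes out and its loop sound mutes.
; Refuelling restores health and restarts the loop.
; Healing goes through an interface on overlap; cooking and dome-scaling logic exist but are disconnected.
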(event `UI_Health_Fire_Displaying`
  ;[1 1 1] Widgets Creation
  (bind _returnvalue (`|CreateWidget` "/Game/UI/Jauges/UI_Health_Fire.UI_Health_Fire_C"))
  (bind _output_get (set `self.REF_UI_Fire_Progress_Bar` _returnvalue))
  (`UserWidget.AddToViewport` _output_get 0))

(event `self.ReceiveBeginPlay`
  (`self.Fix_Origin_LightIntensity and max health`)
  (`self.CreateParameterValue`)
  (`self.Fire_Decrease`)
  (`self.Loop_Fire_Sound_Start`)
  (`self.UI_Health_Fire_Displaying`)
  (`self.UI_Cook_Bar`)
  (bind _asbp_third_person_character (cast `/Game/ThirdPerson/Blueprints/BP_ThirdPersonCharacter` (`GameplayStatics.GetPlayerCharacter` 0)))
  (set `self.REF_Player` _asbp_third_person_character))

(event `UI_Cook_Bar`
  (bind _returnvalue (`|CreateWidget` "/Game/UI/Jauges/UI_Cook_ProgressBar.UI_Cook_ProgressBar_C"))
  (bind _output_get (set `self.REF_CookBar` _returnvalue))
  (`UserWidget.AddToViewport` _output_get 0))

(event `self.ReceiveTick`
  (params (DeltaSeconds :type "Float (single-precision)")))

(event `CreateParameterValue`
  ;[1 1 1] Create Material and Audio Component
  (bind _returnvalue (`KismetMaterialLibrary.CreateDynamicMaterialInstance` (`PrimitiveComponent.GetMaterial` (`self.CampFire`) 0) "MI_TEMP_Camp_Fire"))
  (bind _output_get (set `self.Dynamic Material` _returnvalue))
  (`PrimitiveComponent.SetMaterial` (`self.CampFire`) 0 _output_get)
  (bind _returnvalue_2 (`MaterialInstanceDynamic.K2_GetScalarParameterValue` (`self.Dynamic Material`) "Opacity"))
  (set `self.Original_Emissivness` _returnvalue_2))

(event `Fire_Off`
  ;[1 0.5843 0.3804] Feed_Back_Fire_Off
  (`GameplayStatics.SpawnSoundAtLocation` "/Game/SFX/Fire/Fire_Burst_Flare_01.Fire_Burst_Flare_01" (`SceneComponent.K2_GetComponentLocation` (`self.CampFire`)) (struct) 1.0 1.0 0.0 null null)
  (`self.Loop_Fire_Sound_Decrease`))

(event `Fire_Decrease`
  ;[1 0.3732 0.027] Fire Decrease
  (bind _output_get (set `self.Fire_Health` (- (`self.Fire_Health`) (/ (`GameplayStatics.GetWorldDeltaSeconds`) 1.0))))
  ;;[1 1 1] Collpase
  (set `/Game/UI/Jauges/UI_Health_Fire.HealthFire_Bar` (/ (`self.Fire_Health`) (`self.Fire_Max_Health`)) (`self.REF_UI_Fire_Progress_Bar`))
  (set `/Game/UI/Jauges/UI_Health_Fire.ScoreVIe` (`KismetStringLibrary.Conv_DoubleToString` _output_get) (`self.REF_UI_Fire_Progress_Bar`))
  (`KismetSystemLibrary.Delay` 0.001)
  (`LightComponent.SetIntensity` (`self.Light`) (* (`self.Original_Light_Intensity`) (`KismetMathLibrary.FClamp` (/ (`self.Fire_Health`) (`self.Fire_Max_Health`)))))
  (`self.Feed_BackEmissive_Off`)
  (`self.FireMax_Cap`)
  (if (>= (`self.Fire_Health`) 0.0)
    (`self.Fire_Decrease`)
    (set `self.IsFireOn?` true)
    (else
      (`self.Fire_Off`)
      (set `self.IsFireOn?` false))))

(event `Fire_On`
  ;[1 0.5843 0.3804] Feed_Back_Fire_On
  (`GameplayStatics.SpawnSoundAtLocation` "/Game/SFX/Fire/Fire_Torch_Swoosh_Center_3.Fire_Torch_Swoosh_Center_3" (`SceneComponent.K2_GetComponentLocation` (`self.CampFire`)) (struct) 1.0 1.0 0.0 null null)
  (`self.Loop_Fire_Sound_Increase`))

(event `Fix_Origin_LightIntensity and max health`
  ;[1 1 1] Get All Original Variables
  (set `self.Fire_Max_Health` (`self.Fire_Health`))
  (set `self.Original_Light_Intensity` (`LightComponentBase.Intensity` (`self.Light`)))
  (set `self.Original_Area_Scale` (`SceneComponent.K2_GetComponentScale` (`self.Camp_Area`))))

(event `Loop_Fire_Sound_Start`
  ;[0.4217 1 0.3804] SoundLoop_TurnOn
  (`AddComponent|NODE_AddAudioComponent-5`)
  (bind _returnvalue (`GameplayStatics.SpawnSoundAtLocation` "/Game/SFX/Fire/Fire_Burning_Cracking_Loop_2.Fire_Burning_Cracking_Loop_2" (`SceneComponent.K2_GetComponentLocation` (`self.CampFire`)) (struct) 1.0 1.0 0.0 null null))
  (set `self.NewVar` _returnvalue))

(event `self.FuelFire`
  (params (`IsPlayerFueling?` :type Boolean))
  ;[1 0.628 0] Rechargement de Fuel
  (set `self.IsFireOn?` true)
  (`MaterialInstanceDynamic.SetScalarParameterValue` (`self.Dynamic Material`) (`self.Parameter_Name`) (`self.Original_Emissivness`))
  (`self.Fire_On`)
  (`LightComponent.SetIntensity` (`self.Light`) (`self.Light_Origin`))
  (`self.Combustible_Recharge` (`self.Fire_Max_Health`))
  (`self.Fire_Decrease`))

(event `self.UI_Detector.OnComponentBeginOverlap`
  (params (OverlappedComponent :type "PrimitiveComponent Object Reference") (OtherActor :type "Actor Object Reference") (OtherComp :type "PrimitiveComponent Object Reference") (OtherBodyIndex :type Integer) (bFromSweep :type Boolean) (SweepResult :type "HitResult Structure (by ref)"))
  ;[1 1 1] FireHealth_Displaying
  (`UserWidget.AddToViewport` (`self.REF_UI_Fire_Progress_Bar`) 0))

(event `Loop_Fire_Sound_Decrease`
  ;[0.4217 1 0.3804] SoundTirn_Off
  (`AudioComponent.SetVolumeMultiplier` (`self.NewVar`) 0.0))

(event `self.Camp_Area.OnComponentBeginOverlap`
  (params (OverlappedComponent :type "PrimitiveComponent Object Reference") (OtherActor :type "Actor Object Reference") (OtherComp :type "PrimitiveComponent Object Reference") (OtherBodyIndex :type Integer) (bFromSweep :type Boolean) (SweepResult :type "HitResult Structure (by ref)"))
  ;[0.1442 1 0.1665] Heal_Player (Interfaces)
  (set `self.IsPlayerIntheCamp?` true)
  (if (`KismetSystemLibrary.DoesImplementInterface` OtherActor "/Game/Interfaces/BP_Interfaces_Ennemy.BP_Interfaces_Ennemy_C")
    (if (`self.IsFireOn?`)
      (message `/Game/Interfaces/BP_Interfaces_Ennemy.Heal` OtherActor (`self.Heal_Player`) (`self.Heal_Delay`) false)
      (set `self.Ref_Other Actor` OtherActor))))

(event `self.UI_Detector.OnComponentEndOverlap`
  (params (OverlappedComponent :type "PrimitiveComponent Object Reference") (OtherActor :type "Actor Object Reference") (OtherComp :type "PrimitiveComponent Object Reference") (OtherBodyIndex :type Integer))
  ;[1 1 1] FireHealth_Displaying
)

(event `Loop_Fire_Sound_Increase`
  ;[0.4217 1 0.3804] SoundTirn_Off
  (`AudioComponent.SetVolumeMultiplier` (`self.NewVar`) 1.0))

(event `self.Camp_Area.OnComponentEndOverlap`
  (params (OverlappedComponent :type "PrimitiveComponent Object Reference") (OtherActor :type "Actor Object Reference") (OtherComp :type "PrimitiveComponent Object Reference") (OtherBodyIndex :type Integer))
  ;[1 0.982 0.3033] Stop Healing
  (set `self.IsPlayerIntheCamp?` false)
  (if (`KismetSystemLibrary.DoesImplementInterface` OtherActor "/Game/Interfaces/BP_Interfaces_Ennemy.BP_Interfaces_Ennemy_C")
    (message `/Game/Interfaces/BP_Interfaces_Ennemy.Heal` OtherActor 0.0 0.0 false)))

(event `NightCurseCheck`
  (params (`Night?` :type Boolean))
  ;[0.363 0 0.4583 0.434] Night Curse
  (if (not (`PrimitiveComponent.IsOverlappingActor` (`self.Dome_Collider`) (`self.REF_Player`)))
    (if (`self.REF Is It Night???`)
      (`KismetSystemLibrary.PrintString` "Tu es moaudit !")
      (`/Engine/EditorBlueprintResources/StandardMacros.DoOnce` false :!label _label
        (:`Completed`
          (`/Game/ThirdPerson/Blueprints/BP_ThirdPersonCharacter.Deal_DamagestoPlayer` (`self.REF_Player`) (`self.Night_Curse_Damages`) 0.0)
          (`KismetSystemLibrary.Delay` (`self.Night_Curse_Delay`))
          (goto _label :!via `Reset`))))))

(fn `Combustible_Recharge`
  (params (Fuel_Seconds :type "Float (double-precision)"))
  (bind _ref_other_actor (`self.Ref_Other Actor`))
  (if (`PrimitiveComponent.IsOverlappingActor` (`self.Fuel_Distance`) _ref_other_actor)
    (`KismetSystemLibrary.PrintString` (`KismetSystemLibrary.GetDisplayName` _ref_other_actor))
    (set `self.Fire_Health` (+ (`self.Fire_Health`) Fuel_Seconds))
    (`GameplayStatics.PlaySound2D` null 1.0 1.0 0.0 null null)
    (`self.Fire_On`)))

(fn `Cook`
  (params (Cook_Time :type "Float (double-precision)") (Thing_To_Cook :type "Actor Class Reference"))
  (bind _ref_cookbar (`self.REF_CookBar`))
  (set `self.Original_Cook_Time` Cook_Time)
  (bind _output_get (set `/Game/UI/Jauges/UI_Cook_ProgressBar.CookProgress` (- Cook_Time (/ (`GameplayStatics.GetWorldDeltaSeconds`) 1.0)) _ref_cookbar))
  (if (<= (`/Game/UI/Jauges/UI_Cook_ProgressBar.CookProgress` _ref_cookbar) 0.0)
    (`self.Cook` _output_get)))

(fn `Dome_ComeBack`
  (params (`Entrée` :type "Float (double-precision)"))
  (bind _camp_area (`self.Camp_Area`))
  (`SceneComponent.SetWorldScale3D` _camp_area (`KismetMathLibrary.Conv_DoubleToVector` `Entrée`))
  (`PrimitiveComponent.SetCollisionEnabled` _camp_area "QueryOnly")
  (`KismetSystemLibrary.PrintString` "Dome de retour"))

(fn `Dome_End`
  (params (`Entrée` :type "Float (double-precision)"))
  (bind _camp_area (`self.Camp_Area`))
  (`SceneComponent.SetWorldScale3D` _camp_area (`KismetMathLibrary.Conv_DoubleToVector` `Entrée`))
  (`PrimitiveComponent.SetCollisionEnabled` _camp_area "NoCollision"))

(fn `Feed_BackEmissive_Off`
  (`MaterialInstanceDynamic.SetScalarParameterValue` (`self.Dynamic Material`) (`self.Parameter_Name`) (* (`self.Original_Emissivness`) (/ (`self.Fire_Health`) (`self.Fire_Max_Health`)))))

(fn `FireMax_Cap`
  (bind _fire_max_health (`self.Fire_Max_Health`))
  (if (>= (`self.Fire_Health`) _fire_max_health)
    (set `self.Fire_Health` _fire_max_health)))

(fn `Night_Curse`
  (params (`IsItNight???` :type Boolean))
  (bind _output_get (set `self.REF Is It Night???` `IsItNight???`))
  (`self.NightCurseCheck` _output_get))

(fn `UserConstructionScript`)