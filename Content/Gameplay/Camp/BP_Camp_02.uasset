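; Campfire actor whose fire burns out over time, can be refueled, and sends heal messages to actors overlapping its camp area.
; A timeline paced by FireHealth fades the light and dynamic material, then cuts the looping sound and healing at zero.
; FuelFire relights it, restoring glow and sound and restarting the timeline.
; Tick copies FireHealth, which the timeline never changes, to the health bar widget.
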(event `self.ReceiveBeginPlay`
  (set `self.Fire_Max_Health` (`self.Fire_Health`))
  (bind _ashealth_fire (cast `/Game/UI/Jauges/UI_Health_Fire` (`WidgetComponent.GetUserWidgetObject` (`self.Fire_Health_Bar`))))
  (set `self.REF_UI_Fire_Health` _ashealth_fire)
  (`self.CreateParameterValue`)
  (`self.Temps écoulé`)
  (`self.Loop_Fire_Sound_Start`))

(event `self.ReceiveTick`
  (params (DeltaSeconds :type "Float (single-precision)"))
  (`self.NewFunction`))

(event `UI_Health_Fire_Displaying`
  (bind _returnvalue (`|CreateWidget` "/Game/UI/Jauges/UI_Health_Fire.UI_Health_Fire_C" null 0.0 "" null null))
  (`UserWidget.AddToViewport` _returnvalue 0))

(event `CreateParameterValue`
  ;[1 1 1] Create Material and Audio Component
  (bind _returnvalue (`KismetMaterialLibrary.CreateDynamicMaterialInstance` (`PrimitiveComponent.GetMaterial` (`self.CampFire`) 0) "MI_TEMP_Camp_Fire"))
  (bind _output_get (set `self.Dynamic Material` _returnvalue))
  (`PrimitiveComponent.SetMaterial` (`self.CampFire`) 0 _output_get)
  (bind _returnvalue_2 (`MaterialInstanceDynamic.K2_GetScalarParameterValue` (`self.Dynamic Material`) "Opacity"))
  (set `self.Fire_Recharge` _returnvalue_2))

(event `Fire_Off`
  ;[1 0.5843 0.3804] Feed_Back_Fire_Off
  (`GameplayStatics.SpawnSoundAtLocation` "/Game/SFX/Fire/Fire_Burst_Flare_01.Fire_Burst_Flare_01" (`SceneComponent.K2_GetComponentLocation` (`self.CampFire`)) (struct) 1.0 1.0 0.0 null null)
  (`self.Loop_Fire_Sound_Decrease`))

(event `Temps écoulé`
  (bind _fire_decrease (`self.Fire_Decrease`))
  ;[1 0.3732 0.027] Fire Decrease
  (if (`self.IsFireOn?`)
    (`TimelineComponent.SetPlaybackPosition` _fire_decrease 0.0 false true)
    (`TimelineComponent.SetPlayRate` _fire_decrease (/ 1.0 (`self.Fire_Health`)))
    (bind (_direction _fire_decrease_2) (`Timeline|Fire_Decrease`)
      (:`Update`
        (`LightComponent.SetIntensity` (`self.Light`) (* _fire_decrease_2 2.0))
        (`MaterialInstanceDynamic.SetScalarParameterValue` (`self.Dynamic Material`) (`self.Parameter_Name`) _fire_decrease_2)
        (if (<= _fire_decrease_2 0.0)
          (`self.Fire_Off`)
          (set `self.IsFireOn?` false)
          (message `/Game/Interfaces/BP_Interfaces_Ennemy.Heal` (`self.Ref_Other Actor`) 0.0 0.0 false)
          (elif (>= _fire_decrease_2 0.0)
            _))))))

(event `Fire_On`
  ;[1 0.5843 0.3804] Feed_Back_Fire_On
  (`GameplayStatics.SpawnSoundAtLocation` "/Game/SFX/Fire/Fire_Torch_Swoosh_Center_3.Fire_Torch_Swoosh_Center_3" (`SceneComponent.K2_GetComponentLocation` (`self.CampFire`)) (struct) 1.0 1.0 0.0 null null)
  (`self.Loop_Fire_Sound_Increase`))

(event `/Game/Interfaces/BP_Interfaces_Ennemy.FuelFire`
  (params (`IsPlayerFueling?` :type Boolean))
  ;[0 0 0] Joueur Donne la permission de mettre le fuel
  (`self.Fuel`))

(event `Loop_Fire_Sound_Start`
  ;[0.4217 1 0.3804] SoundTirn_Off
  (`AddComponent|NODE_AddAudioComponent-5`)
  (bind _returnvalue (`GameplayStatics.SpawnSoundAtLocation` "/Game/SFX/Fire/Fire_Burning_Cracking_Loop_2.Fire_Burning_Cracking_Loop_2" (`SceneComponent.K2_GetComponentLocation` (`self.CampFire`)) (struct) 1.0 1.0 0.0 null null))
  (set `self.NewVar` _returnvalue))

(event `Fuel`
  ;[1 0.628 0] Rechargement de Fuel
  (set `self.IsFireOn?` true)
  (`MaterialInstanceDynamic.SetScalarParameterValue` (`self.Dynamic Material`) (`self.Parameter_Name`) (`self.Fire_Recharge`))
  (`self.Fire_On`)
  (`LightComponent.SetIntensity` (`self.Light`) (`self.Light_Origin`))
  (set `self.Is Player Fueling?` false)
  (`self.Temps écoulé`))

(event `Loop_Fire_Sound_Decrease`
  ;[0.4217 1 0.3804] SoundTirn_Off
  (`AudioComponent.SetVolumeMultiplier` (`self.NewVar`) 0.0))

(event `self.Camp_Area.OnComponentBeginOverlap`
  (params (OverlappedComponent :type "PrimitiveComponent Object Reference") (OtherActor :type "Actor Object Reference") (OtherComp :type "PrimitiveComponent Object Reference") (OtherBodyIndex :type Integer) (bFromSweep :type Boolean) (SweepResult :type "HitResult Structure (by ref)"))
  ;[0.1442 1 0.1665] Heal_Player (Interfaces)
  (if (`KismetSystemLibrary.DoesImplementInterface` OtherActor "/Game/Interfaces/BP_Interfaces_Ennemy.BP_Interfaces_Ennemy_C")
    _
    (else
      _))
  (message `/Game/Interfaces/BP_Interfaces_Ennemy.Heal` OtherActor (`self.Heal_Player`) (`self.Heal_Delay`) (`self.IsFireOn?`))
  (set `self.Ref_Other Actor` OtherActor))

(event `Loop_Fire_Sound_Increase`
  ;[0.4217 1 0.3804] SoundTirn_Off
  (`AudioComponent.SetVolumeMultiplier` (`self.NewVar`) 1.0))

(event `self.Camp_Area.OnComponentEndOverlap`
  (params (OverlappedComponent :type "PrimitiveComponent Object Reference") (OtherActor :type "Actor Object Reference") (OtherComp :type "PrimitiveComponent Object Reference") (OtherBodyIndex :type Integer))
  ;[1 1 1] Arrêtte le heal une fois sorti (Je sais pas si ca marche comme il faut)
  (if (`KismetSystemLibrary.DoesImplementInterface` OtherActor "/Game/Interfaces/BP_Interfaces_Ennemy.BP_Interfaces_Ennemy_C")
    (message `/Game/Interfaces/BP_Interfaces_Ennemy.Heal` OtherActor 0.0 0.0 false)))

(fn `NewFunction`
  (returns (NewParam :type "/Game/Gameplay/Camp/BP_Camp_02 Object Reference"))
  (set `/Game/UI/Jauges/UI_Health_Fire.Health` (`self.Fire_Health`) (`self.REF_UI_Fire_Health`))
  (return null))

(fn `UserConstructionScript`)