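; Torch for the camp whose fire gradually dies out during play.
; On BeginPlay it creates a dynamic material for the CampFire mesh, then, if the fire is on, runs a timeline scaled by FireHealth.
; The timeline curve drives both light intensity and a material scalar parameter.
; When the curve reaches zero, the fire is flagged off and its fire-off event is called for sound feedback.
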(event `self.ReceiveBeginPlay`
  (`self.CreateParameterValue`)
  (`self.Temps écoulé`))

(event `CreateParameterValue`
  ;[1 1 1] Create Material
  (bind _returnvalue (`KismetMaterialLibrary.CreateDynamicMaterialInstance` (`PrimitiveComponent.GetMaterial` (`self.CampFire`) 0) "MI_TEMP_Camp_Fire"))
  (bind _output_get (set `self.Dynamic Material` _returnvalue))
  (`PrimitiveComponent.SetMaterial` (`self.CampFire`) 0 _output_get))

(event `Fire_Off`
  ;[1 0.5843 0.3804] Feed_Back_Fire_Off
  (`GameplayStatics.SpawnSoundAtLocation` "/Game/SFX/Fire/Fire_Burst_Flare_01.Fire_Burst_Flare_01" (`SceneComponent.K2_GetComponentLocation` (`self.CampFire`)) (struct) 1.0 1.0 0.0 null null))

(event `Temps écoulé`
  (bind _fire_decrease (`self.Fire_Decrease`))
  ;[1 0.3732 0.027] Fire Decrease
  (if (`self.IsFireOn?`)
    (`TimelineComponent.SetPlaybackPosition` _fire_decrease 0.0 false true)
    (`TimelineComponent.SetPlayRate` _fire_decrease (/ 1.0 (`self.Fire_Health`)))
    (bind (_direction _fire_decrease_2) (`Timeline|Fire_Decrease`)
      (:`Update`
        (`LightComponent.SetIntensity` (`self.Light`) (* _fire_decrease_2 2.0))
        (`MaterialInstanceDynamic.SetScalarParameterValue` (`self.Dynamic Material`) (`self.Parameter_Name`) _fire_decrease_2)
        (if (<= _fire_decrease_2 0.0)
          (`self.Fire_Off`)
          (set `self.IsFireOn?` false)
          (elif (>= _fire_decrease_2 0.0)
            _))))))

(fn `UserConstructionScript`)